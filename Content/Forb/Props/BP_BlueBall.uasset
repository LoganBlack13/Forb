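; BP_BlueBall is a prop with a Sphere component whose physics simulation and gravity can be switched on and off.
; BeginPlay applies the SimulationActive and GravityActive flags to the sphere and enables player 0 input if CanBeControlled is set.
; The IA_ActiveSimulation input action toggles physics simulation at runtime.
; ToggleGravity flips gravity and returns the new state, but nothing in this Blueprint calls it.
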(event Input|EnhancedActionEvents|EnhancedInputActionIA_ActiveSimulation
  (params (ActionValue :type Boolean) (ElapsedSeconds :type Float%20%28double-precision%29) (TriggeredSeconds :type Float%20%28double-precision%29) (InputAction :type Input%20Action%20Object%20Reference :default "/Game/Forb/Core/Inputs/IA_ActiveSimulation.IA_ActiveSimulation"))
  (:Triggered
    (CallFunction|ToggleSimulation)))

(event EventBeginPlay
  (if (Variables|Default|GetbCanBeControlled)
    (Input|EnableInput (Game|GetPlayerController 0)))
  (CallFunction|SetPhysicsSimulation)
  (CallFunction|SetGravity))

(fn ConstructionScript)

(fn ToggleGravity
  (Physics|SetEnableGravity (Variables|Default|GetSphere) (not (Variables|Default|GetbGravityActive)))
  (bind _output_get (Variables|Default|SetbGravityActive (not (Variables|Default|GetbGravityActive))))
  (return _output_get))

(fn ToggleSimulation
  (Physics|SetSimulatePhysics (Variables|Default|GetSphere) (not (Variables|Default|GetbSimulationActive)))
  (bind _output_get (Variables|Default|SetbSimulationActive (not (Variables|Default|GetbSimulationActive))))
  (return _output_get))

(fn SetGravity
  (Physics|SetEnableGravity (Variables|Default|GetSphere) (Variables|Default|GetbGravityActive))
  (return))

(fn SetPhysicsSimulation
  (Physics|SetSimulatePhysics (Variables|Default|GetSphere) (Variables|Default|GetbSimulationActive))
  (return))