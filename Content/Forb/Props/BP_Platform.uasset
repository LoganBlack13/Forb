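; BP_Platform is a platform prop whose look and attached component are determined by its Type.
; On BeginPlay it searches DT_ComponentType for the row matching Type, then applies that row's material to the Cube and adds its component class at runtime.
; ChangeType sets a new Type and, only if a type component already exists, destroys it and reruns the lookup.
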(event EventBeginPlay
  (CallFunction|InitComponentType))

(fn ConstructionScript)

(fn InitComponentType
  (bind _outrownames (DataTable|GetDataTableRowNames "/Game/Forb/Core/Data/DT_ComponentType.DT_ComponentType"))
  (for _array_element _outrownames
    (bind _returnvalue (Utilities|GetDataTableRow "/Game/Forb/Core/Data/DT_ComponentType.DT_ComponentType" _array_element)
      (:then
        (if (Utilities|Enum|Equal(Enum) (Variables|Default|GetType) (.Type (Utilities|Struct|BreakSComponentType _returnvalue)))
          (CallFunction|SetMaterial (.Material (Utilities|Struct|BreakSComponentType _returnvalue)))
          (bind _returnvalue_2 (Game|AddComponentbyClass (.Component (Utilities|Struct|BreakSComponentType _returnvalue))))
          (Variables|Default|SetComponentTypeActor _returnvalue_2)
          (return true)))
      (:RowNotFound
        (return false))))
  (return false))

(fn SetMaterial
  (params (Material :type Material%20Instance%20Object%20Reference))
  (Rendering|Material|SetMaterial (Variables|Default|GetCube) 0 Material)
  (return))

(fn ChangeType
  (params (NewType :type EPlatformType%20Enum :default "NewEnumerator0"))
  (Variables|Default|SetType NewType)
  (bind _componenttypeactor (Variables|Default|GetComponentTypeActor)
    (:then
      (Components|DestroyComponent _componenttypeactor)
      (bind _biscomponentinitiated (CallFunction|InitComponentType))
      (return _biscomponentinitiated))
    (:else)))