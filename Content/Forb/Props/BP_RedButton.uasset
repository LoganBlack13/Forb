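; BP_RedButton is a prop button that triggers the player win when something overlaps its trigger area.
; The overlap fires PushRedButton, which switches off the red light and runs a timeline that nudges the button down each update until it passes a Z limit.
; CallPlayerWin follows after a short delay, with no filter on the overlapping actor or guard against repeat triggers.
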(event OnComponentBeginOverlap(TriggerArea)
  (params (OverlappedComponent :type Primitive%20Component%20Object%20Reference) (OtherActor :type Actor%20Object%20Reference) (OtherComp :type Primitive%20Component%20Object%20Reference) (OtherBodyIndex :type Integer) (bFromSweep :type Boolean) (SweepResult :type Hit%20Result%20Structure%20%28by%20ref%29))
  (CallFunction|PushRedButton)
  (Utilities|FlowControl|Delay 0.5)
  (Default|CallPlayerWin))

(event EventBeginPlay)

(event EventPushRedButton
  (bind _redbutton (Variables|Default|GetRedButton))
  (Utilities|FlowControl|Sequence
    (:then_0
      (Timeline|PushButton Play
        (:Update
          (Transformation|AddLocalOffset _redbutton "0.000000,0.000000,-0.100000" false false)
          (if (< (.z (Variables|/Script/Engine.SceneComponent|GetRelativeLocation _redbutton)) 6.0)
            (Timeline|PushButton Stop)))))
    (:then_1
      (Rendering|Components|Light|SetIntensity (Variables|Default|GetRedLight) 0.0))))

(fn ConstructionScript)