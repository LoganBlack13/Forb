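; Actor component that makes its owner's static mesh respond to the mouse, letting BP_Platform owners change type in edit mode.
; On BeginPlay it caches the mesh and default material, then binds click and cursor-over events.
; Each interaction queries edit mode from the player controller: hovering either outlines the mesh or enables owner input and zeroes Emissive.
; Clicking in edit mode applies the selected tool, while unhovering always disables input and outline.
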(event Custom|OnMeshClicked
  (params (TouchedComponent :type Primitive%20Component%20Object%20Reference) (ButtonPressed :type Key%20Structure :default "None"))
  (bind _bisok (CallFunction|ExecuteAction))
  (Variables|Default|SetbIsTypeChanged _bisok))

(event Custom|OnMeshBeginOver
  (params (TouchedComponent :type Primitive%20Component%20Object%20Reference))
  (CallFunction|MouseOvered))

(event Custom|OnMeshEndOver
  (params (TouchedComponent :type Primitive%20Component%20Object%20Reference))
  (CallFunction|MouseUnovered))

(event EventBeginPlay
  (bind _meshcomponent (CallFunction|InitMesh))
  (EventDispatchers|BindEventtoOnClicked _meshcomponent (delegate Custom|OnMeshClicked))
  (EventDispatchers|BindEventtoOnBeginCursorOver _meshcomponent (delegate Custom|OnMeshBeginOver))
  (EventDispatchers|BindEventtoOnEndCursorOver _meshcomponent (delegate Custom|OnMeshEndOver)))

(fn RegisterDefaultMaterial
  (params (MeshComponent :type Static%20Mesh%20Component%20Object%20Reference))
  (Variables|Default|SetDefaultMaterial (Rendering|Material|GetMaterial MeshComponent 0))
  (return))

(fn MouseOvered
  (bind _biseditmode (Variables|Default|GetbIsEditMode))
  (bind _biseditmode_2 (Variables|Default|GetbIsEditMode))
  (Utilities|IsEditMode
    (:then
      ;[0.184 0.8281 0.03019 0.5] In edit mode we can mesh is oultined anbd we can clik and edit it
      (bind _meshcomponent (Utilities|HasValidMesh)
        (:Is%20Valid
          (CallFunction|Outline _meshcomponent true)
          (return true _biseditmode))
        (:Is%20Not%20Valid
          (Development|PrintString "No Mesh Found" true true "(R=1.000000,G=0.006678,B=0.000000,A=1.000000)" 1e+01)
          (return false _biseditmode))))
    (:else
      ;[0.184 0.8281 0.03019 0.5] Edit mode not active so common mouse over interaction
      (CallFunction|EnableInput)
      (bind _meshcomponent_2 (Utilities|HasValidMesh)
        (:Is%20Valid
          (Rendering|Material|SetScalarParameterValueonMaterials _meshcomponent_2 "Emissive" 0.0)
          (return true _biseditmode_2))
        (:Is%20Not%20Valid
          (return false _biseditmode_2))))))

(fn MouseUnovered
  (bind _biseditmode (Variables|Default|GetbIsEditMode))
  ;[0.184 0.8281 0.03019 0.5] What ever mode, you just want to unselect all
  (CallFunction|DisableInput)
  (bind _meshcomponent (Utilities|HasValidMesh)
    (:Is%20Valid
      (CallFunction|Outline _meshcomponent false)
      (return true _biseditmode))
    (:Is%20Not%20Valid
      (Development|PrintString "No Mesh Found" true true "(R=1.000000,G=0.006678,B=0.000000,A=1.000000)" 1e+01)
      (return false _biseditmode))))

(fn EnableInput
  (Input|EnableInput (Components|GetOwner) (Game|GetPlayerController 0))
  (return))

(fn DisableInput
  (Input|DisableInput (Components|GetOwner) (Game|GetPlayerController 0))
  (return))

(fn SetEditMode
  (params (bIsActive :type Boolean))
  (bind _output_get (Variables|Default|SetbIsEditMode bIsActive))
  (return _output_get))

(fn ExecuteAction
  (bind _selectedtool (CallFunction|GetSelectedTool))
  (Utilities|IsEditMode
    (:then
      (bind _asbp_platform (Utilities|Casting|CastToBP_Platform (Components|GetOwner))
        (:then
          (if (Utilities|Enum|NotEqual(Enum) _selectedtool "NewEnumerator3")
            (bind _biscomponentinitiated (Default|ChangeType _asbp_platform _selectedtool))
            (return _biscomponentinitiated)
            (else
              _)))
        (:CastFailed
          _)))
    (:else
      _))
  (return false))

(fn InitMesh
  (bind _returnvalue (Components|GetOwner))
  (bind _returnvalue_2 (Actor|GetComponentbyClass _returnvalue "/Script/Engine.StaticMeshComponent"))
  (Utilities|IsValid _returnvalue_2
    (:Is%20Valid
      (bind _output_get (Variables|Default|SetMeshComponent _returnvalue_2))
      (CallFunction|RegisterDefaultMaterial _output_get)
      (return _output_get))))

(fn IsTypeChanged
  (return (Variables|Default|GetbIsTypeChanged)))