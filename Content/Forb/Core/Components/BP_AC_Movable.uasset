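; Actor component that lets its owning platform be nudged left or right, extending a parent action component.
; MoveRight and MoveLeft inputs offset the owner along its local Y axis by Delta, with sweep.
; Hovering outside edit mode spawns a rotated BP_Arrow indicator next to the owner, and unhovering destroys it.
; On BeginPlay it shrinks the mesh slightly in X and Y.
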(event Input|EnhancedActionEvents|EnhancedInputActionIA_MoveRight
  (params (ActionValue :type Boolean) (ElapsedSeconds :type Float%20%28double-precision%29) (TriggeredSeconds :type Float%20%28double-precision%29) (InputAction :type Input%20Action%20Object%20Reference :default "/Game/Forb/Core/Inputs/IA_MoveRight.IA_MoveRight"))
  (:Triggered
    (CallFunction|MoveRight)))

(event Input|EnhancedActionEvents|EnhancedInputActionIA_MoveLeft
  (params (ActionValue :type Boolean) (ElapsedSeconds :type Float%20%28double-precision%29) (TriggeredSeconds :type Float%20%28double-precision%29) (InputAction :type Input%20Action%20Object%20Reference :default "/Game/Forb/Core/Inputs/IA_MoveLeft.IA_MoveLeft"))
  (:Triggered
    (CallFunction|MoveLeft)))

(event EventBeginPlay
  (|CallParentFunction)
  (CallFunction|ResizePlatform))

(fn ResizePlatform
  (Transformation|SetRelativeScale3D (Variables|Default|GetMeshComponent) "0.950000,0.950000,1.000000")
  (return))

(fn ShowArrows
  (bind _returnvalue (Components|GetOwner))
  (bind _returnvalue_2 (Transformation|GetActorTransform _returnvalue))
  (Utilities|IsValid (Variables|Default|GetArrows)
    (:Is%20Not%20Valid
      (bind _returnvalue_3 (Game|SpawnActorfromClass "/Game/Forb/Core/Blueprints/BP_Arrow.BP_Arrow_C" (Math|Transform|MakeTransform (+ (.location _returnvalue_2) "-75.000000,0.000000,0.000000") (Math|Rotator|CombineRotators (.rotation _returnvalue_2) "0.000000,90.000000,0.000000") (.scale _returnvalue_2)) "Undefined" 0 0))
      (Variables|Default|SetArrows _returnvalue_3)
      (return))))

(fn HideArrows
  (bind _arrows (Variables|Default|GetArrows)
    (:then
      (Actor|DestroyActor _arrows)
      (return))
    (:else)))

(fn MouseOvered
  (bind (_bisok _biseditmode) (|CallParentFunction))
  (if (not _biseditmode)
    (CallFunction|ShowArrows)
    (return _bisok _biseditmode)))

(fn MouseUnovered
  (bind (_bisok _biseditmode) (|CallParentFunction))
  (if (not _biseditmode)
    (CallFunction|HideArrows)
    (return _bisok _biseditmode)))

(fn MoveRight
  (Transformation|AddActorLocalOffset (Components|GetOwner) (Math|Vector|MakeVector 0.0 (Variables|Default|Getdelta) 0.0) true false)
  (return))

(fn MoveLeft
  (Transformation|AddActorLocalOffset (Components|GetOwner) (Math|Vector|MakeVector 0.0 (* (Variables|Default|Getdelta) -1.0) 0.0) true false)
  (return))

(fn ExecuteAction
  (bind _bisok (|CallParentFunction))
  (return _bisok))