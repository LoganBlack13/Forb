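; Actor component that makes its owning platform breakable, with a hammer indicator and a dissolve before destruction.
; Hovering outside edit mode spawns a BP_Hammer offset from the owner, and unhovering removes it.
; The IA_Break input swaps in a dissolve material, disables input and hides the hammer.
; A looping timer then raises the material's DissolveOffset until it completes and the owner actor is destroyed.
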(event Custom|DissolvePlatform
  (Rendering|Material|SetScalarParameterValueonMaterials (Variables|Default|GetMeshComponent) "DissolveOffset" (Variables|Default|GetDelta))
  (bind _output_get (Variables|Default|SetDelta (+ (Variables|Default|GetDelta) (Variables|Default|GetDissolveSpeed))))
  (if (>= _output_get 1.0)
    (Utilities|Time|ClearandInvalidateTimerbyHandle (stale Input|EnhancedActionEvents|EnhancedInputActionIA_Break _returnvalue))
    (CallFunction|BreakPlatform)))

(event Input|EnhancedActionEvents|EnhancedInputActionIA_Break
  (params (ActionValue :type Boolean) (ElapsedSeconds :type Float%20%28double-precision%29) (TriggeredSeconds :type Float%20%28double-precision%29) (InputAction :type Input%20Action%20Object%20Reference :default "/Game/Forb/Core/Inputs/IA_Break.IA_Break"))
  (:Triggered
    (Rendering|Material|SetMaterial (Variables|Default|GetMeshComponent) 0 "/Game/Forb/Assets/Materials/Platform/MI_Dissolve_PlatformBreakable.MI_Dissolve_PlatformBreakable")
    (bind _returnvalue (Utilities|Time|SetTimerbyEvent (delegate Custom|DissolvePlatform) 0.01 true))
    (CallFunction|DisableInput)
    (CallFunction|HideHammer)))

(event EventBeginPlay
  (|CallParentFunction) ; This node is disabled and will not be called.\nDrag off pins to build functionality.
)

(fn ShowHammer
  (bind _returnvalue (Components|GetOwner))
  (bind _returnvalue_2 (Transformation|GetActorTransform _returnvalue))
  (Utilities|IsValid (Variables|Default|GetHammer)
    (:Is%20Not%20Valid
      (bind _returnvalue_3 (Game|SpawnActorfromClass "/Game/Forb/Core/Blueprints/BP_Hammer.BP_Hammer_C" (Math|Transform|MakeTransform (+ (.location _returnvalue_2) "-75.000000,0.000000,0.000000") (.rotation _returnvalue_2) (.scale _returnvalue_2)) "Undefined" 0 0))
      (Variables|Default|SetHammer _returnvalue_3)
      (return))))

(fn HideHammer
  (bind _hammer (Variables|Default|GetHammer))
  (Utilities|IsValid _hammer
    (:Is%20Valid
      (Actor|DestroyActor _hammer)
      (return))))

(fn MouseOvered
  (bind (_bisok _biseditmode) (|CallParentFunction))
  (if (not _biseditmode)
    (CallFunction|ShowHammer)
    (return _bisok _biseditmode)))

(fn MouseUnovered
  (bind (_bisok _biseditmode) (|CallParentFunction))
  (if (not _biseditmode)
    (CallFunction|HideHammer)
    (return _bisok _biseditmode)))

(fn BreakPlatform
  (CallFunction|HideHammer)
  (Actor|DestroyActor (Components|GetOwner))
  (return))

(fn ExecuteAction
  (bind _bisok (|CallParentFunction))
  (return _bisok))