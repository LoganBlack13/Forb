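; BP_AC_Pivotable is an interaction component that lets the player rotate a mesh left and right within limits.
; Enhanced Input actions step MeshComponent's local roll by Delta, tracking CurrentRotate against MinRotate and MaxRotate.
; Outside edit mode, mouse hover spawns a BP_RotateArrow offset from the owner and unhover destroys it.
; The rotation inputs check neither hover nor edit mode, and ExecuteAction only defers to the parent.
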(event Input|EnhancedActionEvents|EnhancedInputActionIA_RotateRight
  (params (ActionValue :type Boolean) (ElapsedSeconds :type Float%20%28double-precision%29) (TriggeredSeconds :type Float%20%28double-precision%29) (InputAction :type Input%20Action%20Object%20Reference :default "/Game/Forb/Core/Inputs/IA_RotateRight.IA_RotateRight"))
  (:Triggered
    (CallFunction|RotateRight)))

(event Input|EnhancedActionEvents|EnhancedInputActionIA_RotateLeft
  (params (ActionValue :type Boolean) (ElapsedSeconds :type Float%20%28double-precision%29) (TriggeredSeconds :type Float%20%28double-precision%29) (InputAction :type Input%20Action%20Object%20Reference :default "/Game/Forb/Core/Inputs/IA_RotateLeft.IA_RotateLeft"))
  (:Triggered
    (CallFunction|RotateLeft)))

(event EventBeginPlay
  (|CallParentFunction) ; This node is disabled and will not be called.\nDrag off pins to build functionality.
)

(fn MouseOvered
  (bind (_bisok _biseditmode) (|CallParentFunction))
  (if (not _biseditmode)
    (CallFunction|ShowArrows)
    (return _bisok _biseditmode)))

(fn ShowArrows
  (bind _returnvalue (Components|GetOwner))
  (bind _returnvalue_2 (Transformation|GetActorTransform _returnvalue))
  (Variables|Default|GetArrows
    (:then)
    (:else
      (bind _returnvalue_3 (Game|SpawnActorfromClass "/Game/Forb/Core/Blueprints/BP_RotateArrow.BP_RotateArrow_C" (Math|Transform|MakeTransform (+ (.location _returnvalue_2) "-75.000000,0.000000,0.000000") (Math|Rotator|CombineRotators (.rotation _returnvalue_2) "0.000000,90.000000,0.000000") (.scale _returnvalue_2)) "Undefined" 0 0))
      (Variables|Default|SetArrows _returnvalue_3)
      (return))))

(fn HideArrows
  (bind _arrows (Variables|Default|GetArrows)
    (:then
      (Actor|DestroyActor _arrows)
      (return))
    (:else)))

(fn MouseUnovered
  (bind (_bisok _biseditmode) (|CallParentFunction))
  (if (not _biseditmode)
    (CallFunction|HideArrows)
    (return _bisok _biseditmode)))

(fn RotateRight
  (if (not (<= (Variables|Default|GetMaxRotate) (Variables|Default|GetCurrentRotate)))
    (Transformation|AddLocalRotation (Variables|Default|GetMeshComponent) (Math|Rotator|MakeRotator (Variables|Default|GetDelta) 0.0 0.0) false false)
    (Variables|Default|SetCurrentRotate (+ (Variables|Default|GetCurrentRotate) (Variables|Default|GetDelta)))
    (return)))

(fn RotateLeft
  (if (not (<= (Variables|Default|GetCurrentRotate) (Variables|Default|GetMinRotate)))
    (Transformation|AddLocalRotation (Variables|Default|GetMeshComponent) (Math|Rotator|MakeRotator (* (Variables|Default|GetDelta) -1.0) 0.0 0.0) false false)
    (Variables|Default|SetCurrentRotate (- (Variables|Default|GetCurrentRotate) (Variables|Default|GetDelta)))
    (return)))

(fn ExecuteAction
  (bind _bisok (|CallParentFunction))
  (return _bisok))