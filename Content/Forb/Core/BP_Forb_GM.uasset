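; Game mode for Forb that boots both the main menu and playable maps and tracks map unlock progress.
; On BeginPlay it loads or creates the save, registers the player controller, input mapping and widgets, then branches on map name.
; The menu's map-selected event opens the chosen level, while other maps show the HUD and any map-specific message.
; The controller's player-won event adds the current map to the unlocked list and saves it.
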(event Custom|LaunchMainMenu
  (bind _mainmenuui (Variables|Default|GetMainMenuUI))
  ;[0.184 0.8281 0.03019 0.5] Main menu management add to viewport and bind map selection
  (UserInterface|Viewport|AddtoViewport _mainmenuui 0)
  (EventDispatchers|BindEventtoMapSelected _mainmenuui (delegate Custom|LaunchMap)))

(event Custom|LaunchMap
  (params (Map :type Name))
  ;[0.184 0.8281 0.03019 0.5] Map selected and opened
  (EventDispatchers|UnbindallEventsfromMapSelected (Variables|Default|GetMainMenuUI))
  (Game|OpenLevel(byName) Map))

(event Custom|PlayerWon
  ;[0.184 0.8281 0.03019 0.5] after player won a map actions like update maps unlock
  (CallFunction|SetMapUnlock (CallFunction|GetCurrentMapName))
  (CallFunction|SaveGame)
  (EventDispatchers|UnbindallEventsfromPlayerWon (Variables|Default|GetPlayerController)))

(event EventBeginPlay
  ;[0.184 0.8281 0.03019 0.5] Save init
  (CallFunction|InitSavegame)
  ;[0.184 0.8281 0.03019 0.5] Start game, register player controller, initialize input mapping, register MainMenu UI and ad correct UI regarding if player is in main menu or in a map
  (bind _playercontroller (CallFunction|RegisterPlayerController))
  (Input|AddMappingContext (PlayerController|LocalPlayerSubsystems|GetEnhancedInputLocalPlayerSubsystem _playercontroller) "/Game/Forb/Core/Inputs/IM_Player.IM_Player" 0 "(bIgnoreAllPressedKeysUntilRelease=True,bForceImmediately=False)")
  (CallFunction|RegisterMainMenu)
  (CallFunction|RegisterHUD)
  (if (== (CallFunction|GetCurrentMapName) "MainMenu")
    (CallFunction|LaunchMainMenu)
    (else
      (Default|SetHUD (Variables|Default|GetPlayerController) (Variables|Default|GetPlayerHUD))
      (CallFunction|InitializePlayerHUD)
      (EventDispatchers|BindEventtoPlayerWon (Variables|Default|GetPlayerController) (delegate Custom|PlayerWon))
      (CallFunction|DisplayMessageFormMap))))

(fn ConstructionScript)

(fn RegisterPlayerController
  (bind _asbp_forb_pc (Utilities|Casting|CastToBP_Forb_PC (Game|GetPlayerController 0)))
  (bind _output_get (Variables|Default|SetPlayerController _asbp_forb_pc))
  (return _output_get))

(fn RegisterMainMenu
  (bind _returnvalue (UserInterface|CreateWidget "/Game/Forb/UI/WBP_MainMenu.WBP_MainMenu_C"))
  (bind _output_get (Variables|Default|SetMainMenuUI _returnvalue))
  (return _output_get))

(fn InitializePlayerHUD
  (bind _playerhud (Variables|/Game/Forb/Core/BP_Forb_PC.BP_Forb_PC_C|GetPlayerHUD (Variables|Default|GetPlayerController))
    (:then
      (UserInterface|Viewport|AddtoViewport _playerhud 0))
    (:else
      (Development|PrintString "HUD not found" true true "(R=1.000000,G=0.006678,B=0.000000,A=1.000000)" 1e+01)))
  (return))

(fn RegisterHUD
  (bind _returnvalue (UserInterface|CreateWidget "/Game/Forb/UI/WBP_HUD.WBP_HUD_C"))
  (bind _output_get (Variables|Default|SetPlayerHUD _returnvalue))
  (return _output_get))

(fn SetMapUnlock
  (params (Map :type Name))
  (Utilities|Array|AddUnique (Variables|Default|GetMapsUnlocked) Map)
  (return))

(fn InitSavegame
  (bind _returnvalue (SaveGame|DoesSaveGameExist (Variables|Default|GetSaveName)))
  (if _returnvalue
    (bind _returnvalue_2 (SaveGame|LoadGamefromSlot (Variables|Default|GetSaveName)))
    (bind _asbp_forb_sg (Utilities|Casting|CastToBP_Forb_SG _returnvalue_2)
      (:then
        (Variables|Default|SetMapsUnlocked (Variables|/Game/Forb/Core/BP_Forb_SG.BP_Forb_SG_C|GetMapsUnlocked _asbp_forb_sg)))
      (:CastFailed
        _))
    (else
      (bind _returnvalue_3 (SaveGame|CreateSaveGameObject "/Game/Forb/Core/BP_Forb_SG.BP_Forb_SG_C"))
      (Variables|/Game/Forb/Core/BP_Forb_SG.BP_Forb_SG_C|SetMapsUnlocked _returnvalue_3 (Variables|Default|GetMapsUnlocked))
      (SaveGame|SaveGametoSlot _returnvalue_3 (Variables|Default|GetSaveName))))
  (return))

(fn SaveGame
  (bind _returnvalue (SaveGame|DoesSaveGameExist (Variables|Default|GetSaveName)))
  (if _returnvalue
    (bind _returnvalue_2 (SaveGame|LoadGamefromSlot (Variables|Default|GetSaveName)))
    (bind _asbp_forb_sg (Utilities|Casting|CastToBP_Forb_SG _returnvalue_2))
    (Variables|/Game/Forb/Core/BP_Forb_SG.BP_Forb_SG_C|SetMapsUnlocked _asbp_forb_sg (Variables|Default|GetMapsUnlocked))
    (SaveGame|SaveGametoSlot _asbp_forb_sg (Variables|Default|GetSaveName))
    (return)
    (else
      (return))))

(fn DisplayMessageFormMap
  (bind _levelname (CallFunction|GetCurrentMapName))
  (bind _mapsmessage (Variables|Default|GetMapsMessage))
  (bind (_value _returnvalue) (Utilities|Map|Find _mapsmessage _levelname))
  (if _returnvalue
    (CallFunction|Notify _value)))