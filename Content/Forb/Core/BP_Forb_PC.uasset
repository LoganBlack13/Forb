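; Player controller that runs each map's win flow and an edit mode for selecting tools.
; On BeginPlay it finds the BP_RedButton and binds its win event, which pauses the game and shows a menu to retry, open the next map in the map list, or return to MainMenu.
; An input action toggles edit mode on editable maps, notifies listeners and binds HUD tool selection, which sets the mouse cursor per tool.
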(event Custom|OnToolSelected
  (params (Tool :type EPlatformType%20Enum :default "NewEnumerator0"))
  ;[0.184 0.8281 0.03019 0.5] Selected tool event
  (CallFunction|SetSelectedTool Tool))

(event Custom|PlayerWin
  (bind _playerhud (Variables|Default|GetPlayerHUD))
  ;[0.184 0.8281 0.03019 0.5] Player win menu and action binding
  (Game|SetGamePaused true)
  (Default|DisplayWinMenu _playerhud)
  (EventDispatchers|BindEventtoRetryMap _playerhud (delegate Custom|RetryMap))
  (EventDispatchers|BindEventtoNextMap _playerhud (delegate Custom|NextMap))
  (EventDispatchers|BindEventtoGotoMainMenu _playerhud (delegate Custom|MainMenu))
  (Default|CallPlayerWon))

(event Custom|RetryMap
  ;[0.184 0.8281 0.03019 0.5] End Map Menu to retry, go next or qui to main menu
  (CallFunction|RetryMap))

(event Custom|NextMap
  ;[0.184 0.8281 0.03019 0.5] End Map Menu to retry, go next or qui to main menu
  (Game|OpenLevel(byName) (CallFunction|GetNextMap)))

(event Custom|MainMenu
  ;[0.184 0.8281 0.03019 0.5] End Map Menu to retry, go next or qui to main menu
  (Game|OpenLevel(byName) "MainMenu"))

(event Input|EnhancedActionEvents|EnhancedInputActionIA_EditModeToggle
  (params (ActionValue :type Boolean) (ElapsedSeconds :type Float%20%28double-precision%29) (TriggeredSeconds :type Float%20%28double-precision%29) (InputAction :type Input%20Action%20Object%20Reference :default "/Game/Forb/Core/Inputs/IA_EditModeToggle.IA_EditModeToggle"))
  (bind _playerhud (Variables|Default|GetPlayerHUD))
  ;[0.184 0.8281 0.03019 0.5] Toggle edit mode and call event to warn listeners
  (:Triggered
    (if (CallFunction|IsMapEditable)
      (bind _output_get (Variables|EditMode|SetbIsEditMode (not (Variables|EditMode|GetbIsEditMode))))
      (if _output_get
        (Default|ToggleEditMenu _playerhud true)
        (EventDispatchers|BindEventtoToolSelected _playerhud (delegate Custom|OnToolSelected))
        (Default|CallEditModeChanged true)
        (else
          (Default|ToggleEditMenu _playerhud false)
          (EventDispatchers|UnbindallEventsfromToolSelected (Variables|Default|GetPlayerHUD))
          (CallFunction|SetSelectedTool "NewEnumerator3")
          (Default|CallEditModeChanged false))))))

(event EventBeginPlay
  ;[0.184 0.8281 0.03019 0.5] Each time Map is open,check if redButton is present  and resiter it, and bind player win event
  (bind _redbutton (CallFunction|RegisterRedButton))
  (Utilities|IsValid _redbutton
    (:Is%20Valid
      (EventDispatchers|BindEventtoPlayerWin (Variables|Default|GetRedButton) (delegate Custom|PlayerWin)))))

(fn ConstructionScript)

(fn SetHUD
  (params (HUD :type WBP%20HUD%20Object%20Reference))
  (bind _output_get (Variables|Default|SetPlayerHUD HUD))
  (return _output_get))

(fn SetSelectedTool
  (params (Tool :type EPlatformType%20Enum :default "NewEnumerator0"))
  (Variables|EditMode|SetSelectedTool Tool)
  (CallFunction|SetMouseCursor)
  (return))

(fn SetMouseCursor
  (switch Utilities|FlowControl|Switch|SwitchonEPlatformType (Variables|EditMode|GetSelectedTool)
    (:NewEnumerator0
      (Variables|Default|SetCurrentMouseCursor "ResizeUpDown"))
    (:NewEnumerator1
      (Variables|Default|SetCurrentMouseCursor "ResizeLeftRight"))
    (:NewEnumerator2
      (Variables|Default|SetCurrentMouseCursor "Hand"))
    (:NewEnumerator3
      (Variables|Default|SetCurrentMouseCursor "Default")))
  (return))

(fn RegisterRedButton
  (bind _outactors (Actor|GetAllActorsOfClass "/Game/Forb/Props/BP_RedButton.BP_RedButton_C"))
  (for _array_element _outactors
    (bind _output_get (Variables|Default|SetRedButton _array_element))
    (return _output_get)))

(fn GetNextMap
  (bind _levelname (CallFunction|GetCurrentMapName))
  (bind _outrownames (CallFunction|GetMapList))
  (bind _returnvalue (Utilities|Array|FindItem _outrownames _levelname))
  (bind _returnvalue_2 (+ _returnvalue 1))
  (if (Utilities|Array|IsValidIndex _outrownames _returnvalue_2)
    (return (Utilities|Array|Get(acopy) _outrownames _returnvalue_2))
    (else
      (return (LocalVariables|GetNoNextMap)))))

(fn IsEditModeActive
  (return (Variables|EditMode|GetbIsEditMode)))